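; Farm plot Blueprint that plants a crop from a struct (corn, pumpkin or carrot presets), grows it and yields a random harvest.
; A looping timer scales up the crop mesh and advances its growth state, or clears its material when rotten.
; Interacting harvests grown crops, otherwise fertilises, then waters.
; Both together shorten the stored grow time, but the running timer keeps its original interval.
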(event `TakenCareoF`
  ;[1 1 1] Taken care of
  (`KismetSystemLibrary.PrintString` "Take care of")
  (if (`KismetMathLibrary.BooleanNAND` (`self.BeenWatered`) (`self.Fertilesed`))
    _))

(event `Root`
  ;[1 1 1] Root
  (`PrimitiveComponent.SetMaterial` (`self.Crop`) 0 null)
  (`KismetSystemLibrary.PrintString` "This wack man"))

(event `Corn`
  ;[1 1 1] Corn
  (`self.Planting` (make `/Game/Blueprints/Struct_crop` "Chair" "/Game/StarterContent/Props/SM_Chair.SM_Chair" "/Engine/MapTemplates/Materials/BasicAsset01.BasicAsset01" (`KismetMathLibrary.MakeTransform` (0.0 0.0 0.0) (struct) (0.3 0.5 0.3)) 5.0 false 0 6 0 100)))

(event `Planting`
  (params (`What crop` :type "/Game/Blueprints/Struct_crop Structure"))
  (bind (_crop_current_growth_state _crop_max_growth_state _crop_minimum_yield _crop_max_yield _crop_is_fully_grown _crop_growtime _crop_starting_size) (`/Game/Blueprints/BML_crops.CROPS_getcropstats` `What crop`))
  (bind (_crop_static_mesh _crop_matieral) (`/Game/Blueprints/BML_crops.CROPS_getcropvisual` `What crop`))
  (bind _crop (`self.Crop`))
  ;[1 1 1] Plant function
  (set `self.Current crop` `What crop`)
  (set `self.Is harvested` false)
  (`KismetSystemLibrary.PrintString` (`KismetStringLibrary.Conv_NameToString` (`/Game/Blueprints/BML_crops.CROPS_getcropname` `What crop`)))
  (`SceneComponent.K2_SetRelativeTransform` _crop _crop_starting_size false false)
  (`StaticMeshComponent.SetStaticMesh` _crop _crop_static_mesh)
  (`PrimitiveComponent.SetMaterial` _crop 0 _crop_matieral)
  (`SceneComponent.SetHiddenInGame` _crop false false)
  (bind _returnvalue (`KismetSystemLibrary.K2_SetTimerDelegate` (delegate `Grow`) _crop_growtime true))
  (`VisualLoggerKismetLibrary.LogText` null "Debug man"))

(event `Plant pumking`
  ;[1 1 1] Pumking
  (`self.Planting` (make `/Game/Blueprints/Struct_crop` "Pumking" "/Engine/Functions/Engine_MaterialFunctions02/ExampleContent/TextureBasedWPO/DemoBoxMesh.DemoBoxMesh" "/Engine/MapTemplates/Materials/BasicAsset01.BasicAsset01" (`KismetMathLibrary.MakeTransform` (0.0 0.0 0.0) (struct) (0.5 0.5 0.5)) 5.0 false 0 6 1)))

(event `Grow`
  (bind (_crop_current_growth_state _crop_max_growth_state _crop_minimum_yield _crop_max_yield _crop_is_fully_grown _crop_growtime) (`/Game/Blueprints/BML_crops.CROPS_getcropstats` (`self.Current crop`)))
  ;[1 1 1] Grow funciton
  (if (`self.Rooten`)
    ;;[1 1 1] new
    (`self.Root`)
    (elif (not _crop_is_fully_grown)
      (`SceneComponent.SetWorldScale3D` (`self.Crop`) (* (`SceneComponent.K2_GetComponentScale` (`self.Crop`)) 1.25))
      (`SceneComponent.SetHiddenInGame` (`self.Crop`) false false)
      (bind _result (`/Engine/EditorBlueprintResources/StandardMacros.IncrementInt` _crop_current_growth_state)
        (:`  `
          (if (and (`self.BeenWatered`) (`self.Fertilesed`))
            (bind _returnvalue (>= _result _crop_max_growth_state))
            (bind _structout (setmembers `/Game/Blueprints/Struct_crop` :`StructRef` (`self.Current crop`) :`Growtime` (/ _crop_growtime 1.4) :`Is fully grown` _returnvalue :`Current growth state` _result))
            (set `self.Current crop` _structout)
            (`KismetSystemLibrary.PrintString` "Crop improved")
            (else
              (bind _structout_2 (setmembers `/Game/Blueprints/Struct_crop` :`StructRef` (`self.Current crop`) :`Growtime` 10.0 :`Is fully grown` _returnvalue :`Current growth state` _result))
              (set `self.Current crop` _structout_2))))))))

(event `Plant carrot`
  ;[1 1 1] Carrot
  (`self.Planting` (make `/Game/Blueprints/Struct_crop` "Carrot" "/Game/FBX/FBX_carrot.FBX_carrot" "/Engine/MapTemplates/Materials/BasicAsset01.BasicAsset01" (`KismetMathLibrary.MakeTransform` (0.0 0.0 -25.0) (struct) (0.4 0.4 0.25)) 10.0 false 0 4 1)))

(event `/Game/Blueprints/BPI_Intreactions.Intract`
  (params (`Who intracted` :type "Actor Object Reference"))
  (bind _current_crop (`self.Current crop`))
  (bind (_crop_current_growth_state _crop_max_growth_state _crop_minimum_yield _crop_max_yield _crop_is_fully_grown) (`/Game/Blueprints/BML_crops.CROPS_getcropstats` _current_crop))
  ;[1 1 1] Harvest with yield
  (if (and (not (`self.Is harvested`)) _crop_is_fully_grown)
    (`SceneComponent.SetHiddenInGame` (`self.Crop`) true false)
    (`KismetSystemLibrary.PrintString` (`KismetStringLibrary.Concat_StrStr` "You harvested " (`KismetStringLibrary.Conv_IntToString` (`KismetMathLibrary.RandomIntegerInRange` _crop_minimum_yield _crop_max_yield)) " " (`KismetStringLibrary.Conv_NameToString` (`/Game/Blueprints/BML_crops.CROPS_getcropname` _current_crop))))
    (set `self.Is harvested` true)
    (`KismetSystemLibrary.K2_ClearAndInvalidateTimerHandle` (stale `Planting` _returnvalue))
    (elif (`self.Fertilesed`)
      (set `self.BeenWatered` true)
      (else
        (bind _output_get (set `self.Fertilesed` true))
        (`KismetSystemLibrary.PrintString` (`KismetStringLibrary.Conv_BoolToString` _output_get))))))

(fn `UserConstructionScript`)
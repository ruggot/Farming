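; Custom player controller that lets the player interact with soil plots by pressing E.
; It caches the pawn on possession, then on E runs a debug-drawn object trace for WorldDynamic objects a short distance forward from that pawn's camera.
; When the hit actor is a Plot_of_Soil, it sends IntractMessage to it, passing the pawn along.
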(event `Key|E`
  (params (Key :type "Key Structure"))
  (bind _returnvalue (`self.GetComponentByClass` (`self.My pawn`) "/Script/Engine.CameraComponent"))
  (bind _returnvalue_2 (`SceneComponent.K2_GetComponentLocation` _returnvalue))
  (:`Pressed`
    (bind (_outhit _returnvalue_3) (`KismetSystemLibrary.LineTraceSingleForObjects` _returnvalue_2 (+ _returnvalue_2 (* (`SceneComponent.GetForwardVector` _returnvalue) 500.0)) (`|MakeArray` "ObjectTypeQuery2" :!type "EObjectTypeQuery Enum") false (`|MakeArray` (`self.My pawn`) :!type "Actor Object Reference") "ForDuration"))
    (cast `/Game/Blueprints/Plot_of_Soil` (`.HitActor` (`GameplayStatics.BreakHitResult` _outhit)))
    (if _returnvalue_3
      (message `/Game/Blueprints/BPI_Intreactions.Intract` (`.HitActor` (`GameplayStatics.BreakHitResult` _outhit)) (`self.My pawn`)))))

(event `self.ReceivePossess`
  (params (PossessedPawn :type "Pawn Object Reference"))
  (set `self.My pawn` PossessedPawn))

(fn `UserConstructionScript`)